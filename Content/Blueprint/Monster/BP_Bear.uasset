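; Bear enemy character that senses, chases and attacks the player, driven by a Locomotion/Chase/Attack/Dead state machine.
; UpdateState mirrors state to the AI Blackboard and sets walk speed; perception starts chases, while Tick drops them on distance or player death during attacks.
; BPHPController handles damage, updating the HP bar and triggering death.
; Toggled collision deals attack damage, and timelines animate material hit flashes and death dissolve before destruction.
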(event OnComponentBeginOverlap(AttackCollision)
  (params (OverlappedComponent :type Primitive%20Component%20Object%20Reference) (OtherActor :type Actor%20Object%20Reference) (OtherComp :type Primitive%20Component%20Object%20Reference) (OtherBodyIndex :type Integer) (bFromSweep :type Boolean) (SweepResult :type Hit%20Result%20Structure%20%28by%20ref%29))
  (Game|Damage|ApplyDamage OtherActor (Variables|Default|GetBase%20Damage) (Pawn|GetController) self))

(event OnTargetPerceptionUpdated(AIPerception)
  (params (Actor :type Actor%20Object%20Reference) (Stimulus :type AI%20Stimulus%20Structure))
  ;[0.15 0.15 0.15 0.5] 시야감지
  (if (.bSuccessfullySensed (Utilities|Struct|BreakAIStimulus Stimulus))
    (if (Utilities|Enum|Equal(Enum) (Variables|Default|GetState_BP) "NewEnumerator0")
      (if (Actor|ActorHasTag Actor "Player")
        (AI|Components|Blackboard|SetValueasObject (Variables|/Script/AIModule.AIController|GetBlackboard (AI|GetAIController self)) (Variables|Default|GetTargetPlayerKey) Actor)
        ;;[0.15 0.15 0.15 0.5] 플레이어 죽었는지 확인
        (bind _asbp_character (Utilities|Casting|CastToBP_Character Actor))
        (if (not (Utilities|Enum|Equal(Enum) (Variables|/Game/Blueprint/Charater/BP_Character.BP_Character_C|GetState_BP _asbp_character) "NewEnumerator2"))
          (CallFunction|UpdateState "NewEnumerator1"))))))

(event OnPerceptionUpdated(AIPerception)
  (params (UpdatedActors :type Array%20of%20Actor%20Object%20References)))

(event Custom|ReceiveOnDead
  (bind _mesh (Variables|Character|GetMesh))
  ;[0.15 0.15 0.15 0.5] 죽은 이벤트 바인딩
  (CallFunction|UpdateState "NewEnumerator3")
  (Collision|SetCollisionEnabled (Variables|Collision|GetCapsuleComponent) "NoCollision")
  (Utilities|FlowControl|Delay 2.0)
  (bind (_direction _dissolve _hitvalue) (Timeline|DeathEffect PlayFromStart)
    (:Update
      (Rendering|Material|SetScalarParameterValueonMaterials _mesh "Dissolve" _dissolve)
      (Rendering|Material|SetScalarParameterValueonMaterials _mesh "HitValue" _hitvalue))
    (:Finished
      (Actor|DestroyActor))))

(event Custom|UpdateState
  (params (NewState :type EBearState%20Enum :default "NewEnumerator0"))
  (bind _charactermovement (Variables|Character|GetCharacterMovement))
  ;[0.15 0.15 0.15 0.5] 상태 변경 이벤트
  (if (Utilities|Enum|NotEqual(Enum) (Variables|Default|GetState_BP) "NewEnumerator3")
    (bind _output_get (Variables|Default|SetState_BP NewState))
    (AI|Components|Blackboard|SetValueasEnum (Variables|/Script/AIModule.AIController|GetBlackboard (AI|GetAIController self)) (Variables|Default|GetStateKey) _output_get)
    (switch Utilities|FlowControl|Switch|SwitchonEBearState (Variables|Default|GetState_BP)
      (:NewEnumerator0
        (Variables|/Script/Engine.CharacterMovementComponent|SetMaxWalkSpeed _charactermovement 2e+02))
      (:NewEnumerator1
        (Variables|/Script/Engine.CharacterMovementComponent|SetMaxWalkSpeed _charactermovement 5e+02))
      (:NewEnumerator2
        (Variables|/Script/Engine.CharacterMovementComponent|SetMaxWalkSpeed _charactermovement 0.0 :!label _label))
      (:NewEnumerator3
        (goto _label)))))

(event Custom|OnAttackCheckStart
  (Collision|SetCollisionEnabled (Variables|Default|GetAttackCollision) "QueryOnly"))

(event Custom|OnAttackCheckEnd
  (Collision|SetCollisionEnabled (Variables|Default|GetAttackCollision) "NoCollision"))

(event Custom|ReciveOnHpChanged
  (params (HealthPower :type Float%20%28double-precision%29) (MaxHealthPower :type Float%20%28double-precision%29))
  ;[0.15 0.15 0.15 0.5] 죽은 이벤트 바인딩
  (bind _aswbp_hpbar (Utilities|Casting|CastToWBP_HPBar (UserInterface|GetUserWidgetObject (Variables|Default|GetHPBar))))
  (Default|UpdateHpPercent _aswbp_hpbar (/ HealthPower MaxHealthPower)))

(event EventBeginPlay
  ;[0.15 0.15 0.15 0.5] 죽은 이벤트 바인딩
  (EventDispatchers|BindEventtoOnDeadEvent (Variables|Default|GetBP_HP_Controller) (delegate Custom|ReceiveOnDead))
  (Collision|SetCollisionEnabled (Variables|Default|GetAttackCollision) "NoCollision")
  (EventDispatchers|BindEventtoOnHpChanged (Variables|Default|GetBP_HP_Controller) (delegate Custom|ReciveOnHpChanged)))

(event Collision|EventActorBeginOverlap
  (params (OtherActor :type Actor%20Object%20Reference))
  (if (Actor|ActorHasTag OtherActor "PlayerWeapon")
    (bind _hitvalue (Timeline|Timeline PlayFromStart)
      (:Update
        (Rendering|Material|SetScalarParameterValueonMaterials (Variables|Character|GetMesh) "HitValue" _hitvalue)))))

(event Game|Damage|EventAnyDamage
  (params (Damage :type Float%20%28single-precision%29) (DamageType :type Damage%20Type%20Object%20Reference) (InstigatedBy :type Controller%20Object%20Reference) (DamageCauser :type Actor%20Object%20Reference))
  (CallFunction|TurntoTarget DamageCauser)
  (Default|ReceiveDamage (Variables|Default|GetBP_HP_Controller) Damage))

(event EventTick
  (params (DeltaSeconds :type Float%20%28single-precision%29))
  (switch Utilities|FlowControl|Switch|SwitchonEBearState (Variables|Default|GetState_BP)
    (:NewEnumerator0
      (CallFunction|OnLocomotion))
    (:NewEnumerator1
      (CallFunction|OnChase))
    (:NewEnumerator2
      (CallFunction|OnAttack))
    (:NewEnumerator3
      (CallFunction|OnDead))))

(fn ConstructionScript)

(fn OnChase
  (bind _asactor (Utilities|Casting|CastToActor (AI|Components|Blackboard|GetValueasObject (Variables|/Script/AIModule.AIController|GetBlackboard (AI|GetAIController self)) (Variables|Default|GetTargetPlayerKey))))
  (if (> (Math|Vector|Distance(Vector) (Transformation|GetActorLocation _asactor) (Transformation|GetActorLocation)) 4e+02)
    (CallFunction|UpdateState "NewEnumerator0")))

(fn OnLocomotion)

(fn OnAttack
  (bind _asbp_character (Utilities|Casting|CastToBP_Character (AI|Components|Blackboard|GetValueasObject (AI|GetBlackboard (AI|GetAIController self)) (Variables|Default|GetTargetPlayerKey))))
  ;[0.15 0.15 0.15 0.5] 플레이어가 죽었는지 확인
  (if (Utilities|Enum|Equal(Enum) (Variables|/Game/Blueprint/Charater/BP_Character.BP_Character_C|GetState_BP _asbp_character) "NewEnumerator2")
    (CallFunction|UpdateState "NewEnumerator0")))

(fn OnDead)

(fn TurntoTarget
  (params (Target :type Actor%20Object%20Reference))
  (Transformation|SetActorRotation (Math|Conversions|RotationFromXVector (- (Transformation|GetActorLocation Target) (Transformation|GetActorLocation)))))