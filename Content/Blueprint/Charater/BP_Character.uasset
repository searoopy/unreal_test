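; Player character Blueprint with Enhanced Input move and look, weapon pickup, combo melee attacks and death handling.
; A state variable gates movement and attacks, while the current montage section determines the next combo.
; Collected weapons attach to a mesh socket and receive attack-check begin/end through event dispatchers.
; Damage feeds HPController and a timeline-driven material hit effect, and its death event disables capsule collision and sets Dead.
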(event Custom|AttackEnd
  (Variables|Default|SetState_BP "NewEnumerator0"))

(event Custom|OnWeaponCollected
  (params (WeaponActor :type BP%20Weapon%20Object%20Reference))
  ;[0.15 0.15 0.15 0.5] 무기 습득 처리
  (Actor|SetOwner WeaponActor self)
  (Transformation|AttachComponentToComponent WeaponActor (Variables|Character|GetMesh) "WeaponPosition" "SnapToTarget" "SnapToTarget" "SnapToTarget" true)
  (Variables|Default|SetWeaponActor WeaponActor)
  (Variables|Default|SetHasWeapon true)
  ;[0.15 0.15 0.15 0.5] 공격판정 시작 이벤트에 함수 등록(구독)
  (EventDispatchers|BindEventtoAttackCheckBeginEvent (delegate Custom|RaiseAttackCheckBegin))
  ;[0.15 0.15 0.15 0.5] 공격판정 종료 이벤트에 함수 등록(구독)
  (EventDispatchers|BindEventtoAttackCheckEndEvent (delegate Custom|RaiseAttackCheckEnd)))

(event Custom|OnAttackCheckBegin
  ;[0.15 0.15 0.15 0.5] 공격판정 시작
  (Default|CallAttackCheckBeginEvent))

(event Custom|OnAttackCheckEnd
  ;[0.15 0.15 0.15 0.5] 공격판정 종료
  (Default|CallAttackCheckEndEvent))

(event Custom|RaiseAttackCheckBegin
  ;[0.15 0.15 0.15 0.5] 공격판정 시작 이벤트에 함수 등록(구독)
  (Utilities|IsValid (Variables|Default|GetWeaponActor)
    (:Is%20Valid
      (Default|OnAttackCheckBegin (Variables|Default|GetWeaponActor)))))

(event Custom|RaiseAttackCheckEnd
  ;[0.15 0.15 0.15 0.5] 공격판정 종료 이벤트에 함수 등록(구독)
  (Utilities|IsValid (Variables|Default|GetWeaponActor)
    (:Is%20Valid
      (Default|OnAttackCheckEnd (Variables|Default|GetWeaponActor)))))

(event Custom|ReceiveOnDeadEvent
  ;[0.15 0.15 0.15 0.5] 죽음 이벤트에 바인딩
  (Collision|SetCollisionEnabled (Variables|Collision|GetCapsuleComponent) "NoCollision")
  (Variables|Default|SetState_BP "NewEnumerator2"))

(event Input|EnhancedActionEvents|EnhancedInputActionIA_Move
  (params (ActionValue :type Vector%202D%20Structure) (ElapsedSeconds :type Float%20%28double-precision%29) (TriggeredSeconds :type Float%20%28double-precision%29) (InputAction :type Input%20Action%20Object%20Reference :default "/Game/Blueprint/Input/Actions/IA_Move.IA_Move"))
  ;[0.15 0.15 0.15 0.5] 이동
  (switch Utilities|FlowControl|Switch|SwitchonEPlayerState (Variables|Default|GetState_BP)
    (:NewEnumerator0
      (Pawn|Input|AddMovementInput (Math|Vector|GetRightVector (Pawn|GetControlRotation :!class /Script/Engine.Pawn)) (.x ActionValue) false)
      (Pawn|Input|AddMovementInput (Math|Vector|GetForwardVector (Math|Rotator|MakeRotator 0.0 0.0 (.yaw (Pawn|GetControlRotation :!class /Script/Engine.Pawn)))) (.y ActionValue) false))))

(event Input|EnhancedActionEvents|EnhancedInputActionIA_View
  (params (ActionValue :type Vector%202D%20Structure) (ElapsedSeconds :type Float%20%28double-precision%29) (TriggeredSeconds :type Float%20%28double-precision%29) (InputAction :type Input%20Action%20Object%20Reference :default "/Game/Blueprint/Input/Actions/IA_View.IA_View"))
  ;[0.15 0.15 0.15 0.5] 회전
  (Pawn|Input|AddControllerYawInput (.x ActionValue)) ; 컨트롤러에 요(yaw)회전 추가
  (Pawn|Input|AddControllerPitchInput (.y ActionValue)) ; 컨트롤러에 피치(pitch)회전 추가
)

(event Input|EnhancedActionEvents|EnhancedInputActionIA_ATTACK
  (params (ActionValue :type Boolean) (ElapsedSeconds :type Float%20%28double-precision%29) (TriggeredSeconds :type Float%20%28double-precision%29) (InputAction :type Input%20Action%20Object%20Reference :default "/Game/Blueprint/Input/Actions/IA_ATTACK.IA_ATTACK"))
  ;[0.15 0.15 0.15 0.5] 공격
  (:Started
    (if (Variables|Default|GetHasWeapon)
      ;;[0.15 0.15 0.15 0.5] 일반상태인지검사
      (switch Utilities|FlowControl|Switch|SwitchonEPlayerState (Variables|Default|GetState_BP)
        (:NewEnumerator0
          (Variables|Default|SetState_BP "NewEnumerator1")
          (Animation|PlayAnimMontage "/Game/Blueprint/Charater/AM_Attack.AM_Attack" 1.0 "None"))
        (:NewEnumerator1
          (switch name (Animation|Montage|MontageGetCurrentSection (Components|SkeletalMesh|GetAnimInstance (Variables|Character|GetMesh)) "/Game/Blueprint/Charater/AM_Attack.AM_Attack")
            (:Attack1
              (Variables|Default|SetNextCombo "Attack2"))
            (:Attack2
              (Variables|Default|SetNextCombo "Attack3"))
            (:Attack3
              (Variables|Default|SetNextCombo "Attack4"))))))))

(event EventBeginPlay
  ;[0.15 0.15 0.15 0.5] 죽음 이벤트에 바인딩
  (EventDispatchers|BindEventtoOnDeadEvent (Variables|Default|GetHP_Controller) (delegate Custom|ReceiveOnDeadEvent)))

(event Collision|EventActorBeginOverlap
  (params (OtherActor :type Actor%20Object%20Reference)))

(event EventTick
  (params (DeltaSeconds :type Float%20%28single-precision%29)))

(event Game|Damage|EventAnyDamage
  (params (Damage :type Float%20%28single-precision%29) (DamageType :type Damage%20Type%20Object%20Reference) (InstigatedBy :type Controller%20Object%20Reference) (DamageCauser :type Actor%20Object%20Reference))
  ;[0.15 0.15 0.15 0.5] 체력 관리 컴퓨넌트 데미지 전달
  (Default|ReceiveDamage (Variables|Default|GetHP_Controller) Damage)
  (bind _hitvalue (Timeline|HitEffect PlayFromStart)
    (:Update
      (Rendering|Material|SetScalarParameterValueonMaterials (Variables|Character|GetMesh) "HitValue" _hitvalue))))

(fn ConstructionScript)